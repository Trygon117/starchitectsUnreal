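; roidField is a Blueprint that scatters an asteroid field as instances of a single instanced static mesh.
; Its construction script adds instances in local space at random directions and distances within a min-max shell around the actor.
; Each gets a random rotation and a uniform random scale adjusted by a multiplier, with count and ranges set by variables.
; The event graph holds no logic.
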(fn `UserConstructionScript`
  (for _ (range (+ (`self.TotalRoids`) 1))
    (`InstancedStaticMeshComponent.AddInstance` (`self.InstancedStaticMesh`) (`KismetMathLibrary.MakeTransform` (* (`KismetMathLibrary.RandomUnitVector`) (`KismetMathLibrary.RandomFloatInRange` (`self.MinDistance`) (`self.MaxDistance`))) (`KismetMathLibrary.RandomRotator` false) (`KismetMathLibrary.Conv_DoubleToVector` (* (`KismetMathLibrary.RandomFloatInRange` (`self.MinScale`) (`self.MaxScale`)) (`self.ScaleMultiplyer`)))) false)))